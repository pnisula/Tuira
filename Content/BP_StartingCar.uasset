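; Car actor that plays a start sound and pops its trunk open to throw out a clothing item when the TopDownCharacter comes near.
; One overlap sphere plays the sound on each entry; the other fires once, rotating the trunk and calling IncreaseEnergyDepletion on the character.
; It spawns SpawnableItem at an arrow, then casts through beanie, mittens, jacket and pants to launch it along the arrow with a short lifespan.
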(event `self.Sphere.OnComponentBeginOverlap`
  (params (OverlappedComponent :type "PrimitiveComponent Object Reference") (OtherActor :type "Actor Object Reference") (OtherComp :type "PrimitiveComponent Object Reference") (OtherBodyIndex :type Integer) (bFromSweep :type Boolean) (SweepResult :type "HitResult Structure (by ref)"))
  (cast `/Game/TopDownCPP/Blueprints/TopDownCharacter` OtherActor)
  (`GameplayStatics.PlaySoundAtLocation` "/Game/Car_Start.Car_Start" (`SceneComponent.K2_GetComponentLocation` (`self.Car`)) (struct) 1.0 1.0 0.0 null null null))

(event `self.Sphere1.OnComponentBeginOverlap`
  (params (OverlappedComponent :type "PrimitiveComponent Object Reference") (OtherActor :type "Actor Object Reference") (OtherComp :type "PrimitiveComponent Object Reference") (OtherBodyIndex :type Integer) (bFromSweep :type Boolean) (SweepResult :type "HitResult Structure (by ref)"))
  (if (not (`self.trunkOpen`))
    (bind _astop_down_character (cast `/Game/TopDownCPP/Blueprints/TopDownCharacter` OtherActor))
    (set `self.trunkOpen` true)
    (`SceneComponent.K2_AddLocalRotation` (`self.Kontti`) (struct :`Pitch` 60.0) false false)
    (`/Game/TopDownCPP/Blueprints/TopDownCharacter.IncreaseEnergyDepletion` _astop_down_character (`self.IncreaseEnergyDepletionTime`))
    (bind _returnvalue (`|SpawnActorFromClass` (`self.SpawnableItem`) (`KismetMathLibrary.Conv_VectorToTransform` (`SceneComponent.K2_GetComponentLocation` (`self.Arrow`))) "Undefined" "OverrideRootScale" null null))
    (bind _asbp_beanie (cast `/Game/Blueprints/BP_Beanie` _returnvalue)
      (:`then`
        (`PrimitiveComponent.AddImpulse` (`/Game/Blueprints/BP_Beanie.Clothes_Beanie` _asbp_beanie) (* (`SceneComponent.GetForwardVector` (`self.Arrow`)) (`self.ThrowForce`)) "None" false)
        (`self.SetLifeSpan` _returnvalue 2.0))
      (:`CastFailed`
        (bind _asbp_mittens (cast `/Game/Blueprints/BP_Mittens` _returnvalue)
          (:`then`
            (`PrimitiveComponent.AddImpulse` (`/Game/Blueprints/BP_Mittens.Clothes_Mittens` _asbp_mittens) (* (`SceneComponent.GetForwardVector` (`self.Arrow`)) (`self.ThrowForce`)) "None" false)
            (`self.SetLifeSpan` _asbp_mittens 2.0))
          (:`CastFailed`
            (bind _asbp_jacket (cast `/Game/Blueprints/BP_Jacket` _returnvalue)
              (:`then`
                (`PrimitiveComponent.AddImpulse` (`/Game/Blueprints/BP_Jacket.Clothes_Jacket` _asbp_jacket) (* (`SceneComponent.GetForwardVector` (`self.Arrow`)) (`self.ThrowForce`)) "None" false)
                (`self.SetLifeSpan` _asbp_jacket 2.0))
              (:`CastFailed`
                (bind _asbp_pants (cast `/Game/Blueprints/BP_Pants` _returnvalue))
                (`PrimitiveComponent.AddImpulse` (`/Game/Blueprints/BP_Pants.Clothes_Pants` _asbp_pants) (* (`SceneComponent.GetForwardVector` (`self.Arrow`)) (`self.ThrowForce`)) "None" false)
                (`self.SetLifeSpan` _asbp_pants 2.0)))))))))

(fn `UserConstructionScript`)