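; Level generator actor that builds a grid of tiles from randomly tall instanced meshes in its construction script.
; Nested loops over Rows and Columns place four objects at offsets around each tile center, each in its own Hierarchical Instanced Static Mesh component.
; One diagonal pair uses the full height scale range, the other half of it.
; One hardcoded tile is left empty, and GetSpawnPointCenter is an unimplemented stub.
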(fn `GetSpawnPointCenter`
  (returns (ReturnValue :type "Transform Structure")))

(fn `UserConstructionScript`
  (bind _returnvalue (/ (`self.Columns`) 2))
  (bind _returnvalue_2 (/ (`self.Rows`) 2))
  (bind _result (`/Engine/EditorBlueprintResources/StandardMacros.NegateInt` _returnvalue_2)
    (:`  `
      (for _index (range _result (+ _returnvalue_2 1))
        (bind _result_2 (`/Engine/EditorBlueprintResources/StandardMacros.NegateInt` _returnvalue)
          (:`  `
            (for _index_2 (range _result_2 (+ _returnvalue 1))
              (if (not (and (== _index 8) (== _index_2 8)))
                (`|ExecutionSequence`
                  (:`then_0`
                    (bind (_returnvalue_x _returnvalue_y) (`KismetMathLibrary.BreakVector` (`KismetMathLibrary.MakeVector` (`KismetMathLibrary.Conv_IntToDouble` (* _index (`self.SpaceBetweenTiles`))) (`KismetMathLibrary.Conv_IntToDouble` (* _index_2 (`self.SpaceBetweenTiles`))))))
                    (`InstancedStaticMeshComponent.AddInstance` (`self.HierarchicalInstancedStaticMesh`) (`KismetMathLibrary.MakeTransform` (`KismetMathLibrary.MakeVector` (- _returnvalue_x (`KismetMathLibrary.Conv_IntToDouble` (`self.SpaceBetweenTileObjects`))) (- _returnvalue_y (`KismetMathLibrary.Conv_IntToDouble` (`self.SpaceBetweenTileObjects`)))) (struct) (`KismetMathLibrary.MakeVector` 1.0 1.0 (`KismetMathLibrary.RandomFloatInRange` (`self.MinHeightOfObjects`) (`self.MaxHeightOfObjects`))))))
                  (:`then_1`
                    (`InstancedStaticMeshComponent.AddInstance` (`self.HierarchicalInstancedStaticMesh1`) (`KismetMathLibrary.MakeTransform` (`KismetMathLibrary.MakeVector` (+ _returnvalue_x (`KismetMathLibrary.Conv_IntToDouble` (`self.SpaceBetweenTileObjects`))) (- _returnvalue_y (`KismetMathLibrary.Conv_IntToDouble` (`self.SpaceBetweenTileObjects`)))) (struct) (`KismetMathLibrary.MakeVector` 1.0 1.0 (`KismetMathLibrary.RandomFloatInRange` (/ (`self.MinHeightOfObjects`) 2.0) (/ (`self.MaxHeightOfObjects`) 2.0))))))
                  (:`then_2`
                    (`InstancedStaticMeshComponent.AddInstance` (`self.HierarchicalInstancedStaticMesh2`) (`KismetMathLibrary.MakeTransform` (`KismetMathLibrary.MakeVector` (- _returnvalue_x (`KismetMathLibrary.Conv_IntToDouble` (`self.SpaceBetweenTileObjects`))) (+ _returnvalue_y (`KismetMathLibrary.Conv_IntToDouble` (`self.SpaceBetweenTileObjects`)))) (struct) (`KismetMathLibrary.MakeVector` 1.0 1.0 (`KismetMathLibrary.RandomFloatInRange` (/ (`self.MinHeightOfObjects`) 2.0) (/ (`self.MaxHeightOfObjects`) 2.0))))))
                  (:`then_3`
                    (`InstancedStaticMeshComponent.AddInstance` (`self.HierarchicalInstancedStaticMesh3`) (`KismetMathLibrary.MakeTransform` (`KismetMathLibrary.MakeVector` (+ _returnvalue_x (`KismetMathLibrary.Conv_IntToDouble` (`self.SpaceBetweenTileObjects`))) (+ _returnvalue_y (`KismetMathLibrary.Conv_IntToDouble` (`self.SpaceBetweenTileObjects`)))) (struct) (`KismetMathLibrary.MakeVector` 1.0 1.0 (`KismetMathLibrary.RandomFloatInRange` (`self.MinHeightOfObjects`) (`self.MaxHeightOfObjects`)))))))))))))))